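; BP_FallingPlatform is a platform that drops shortly after BP_ThirdPersonCharacter overlaps its trigger box.
; After a delay, the Cube simulates physics with a rock material for a set duration, then stops and restores its rock-face material.
; A timeline then lerps toward the starting transform and re-arms on finish.
; The lerp Alpha is fixed at zero, so as written the Cube stays where it fell.
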(event OnComponentBeginOverlap(Box)
  (params (OverlappedComponent :type Primitive%20Component%20Object%20Reference) (OtherActor :type Actor%20Object%20Reference) (OtherComp :type Primitive%20Component%20Object%20Reference) (OtherBodyIndex :type Integer) (bFromSweep :type Boolean) (SweepResult :type Hit%20Result%20Structure%20%28by%20ref%29))
  (Utilities|Casting|CastToBP_ThirdPersonCharacter OtherActor)
  (CallFunction|Activate))

(event Custom|Activate
  (if (Variables|Default|GetbIsReady)
    (Variables|Default|SetbIsReady false)
    (Utilities|FlowControl|Delay (Variables|Default|GetActivatedWaitTime))
    (CallFunction|Drop)))

(event Custom|Drop
  (Physics|SetSimulatePhysics (Variables|Default|GetCube) true)
  (Rendering|Material|SetMaterial (Variables|Default|GetCube) 0 "/Game/Kaitlyn/Materials/MI_Rocks.MI_Rocks")
  (Utilities|FlowControl|Delay (Variables|Default|GetFallingDuration))
  (CallFunction|ResetCube))

(event Custom|ResetCube
  (Variables|Default|SetResetTransform (Transformation|GetWorldTransform (Variables|Default|GetCube)))
  (Physics|SetSimulatePhysics (Variables|Default|GetCube) false)
  (Rendering|Material|SetMaterial (Variables|Default|GetCube) 0 "/Game/Kaitlyn/Materials/M_RockFace.M_RockFace")
  (Timeline|GoBackToStart PlayFromStart
    (:Update
      (Transformation|SetWorldLocationAndRotation (Variables|Default|GetCube) (.location (Math|Transform|Lerp(Transform) (Variables|Default|GetResetTransform) (Variables|Default|GetStartingTransform) 0.0)) (.rotation (Math|Transform|Lerp(Transform) (Variables|Default|GetResetTransform) (Variables|Default|GetStartingTransform) 0.0)) false false))
    (:Finished
      (Variables|Default|SetbIsReady true))))

(event EventBeginPlay
  (Variables|Default|SetStartingTransform (Transformation|GetWorldTransform (Variables|Default|GetCube))))

(event Collision|EventActorBeginOverlap
  (params (OtherActor :type Actor%20Object%20Reference)))

(event EventTick
  (params (DeltaSeconds :type Float%20%28single-precision%29)))

(fn ConstructionScript)